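; MusicManagerBP is a music manager that switches between tracks from a configurable list during play.
; On BeginPlay it creates a 2D sound for every track, starts them all muted, then raises the chosen starting track to the music volume.
; Change_Music mutes the current track and unmutes the one at the given index, an instant volume swap with no restart or crossfade.
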(event Custom|Change_Music
  (params (Index%20Of%20Song%20to%20Play :type Integer))
  (bind _music_ref (Variables|Default|GetMusic_Ref))
  (bind _output (Utilities|Array|Get(acopy) _music_ref Index%20Of%20Song%20to%20Play))
  (Audio|Components|Audio|SetVolumeMultiplier (Variables|Default|GetCurrenMusicRef) 0.0 :!class /Script/Engine.AudioComponent)
  (Audio|Components|Audio|SetVolumeMultiplier _output (Variables|Default|Getmusic%20volume) :!class /Script/Engine.AudioComponent)
  (Variables|Default|SetCurrenMusicRef _output))

(event EventBeginPlay
  (bind _music_ref (Variables|Default|GetMusic_Ref))
  (bind _songtoplayonsart (Variables|Default|GetSongtoPlayonSart))
  (bind _output (Utilities|Array|Get(acopy) _music_ref _songtoplayonsart))
  (for _array_element (Variables|Default|GetTrackList)
    (bind _returnvalue (Audio|CreateSound2D _array_element 1.0 1.0 0.0 0))
    (Utilities|Array|Add (Variables|Default|GetMusic_Ref) _returnvalue)
    (Audio|Components|Audio|SetVolumeMultiplier _returnvalue 0.0 :!class /Script/Engine.AudioComponent)
    (Audio|Components|Audio|Play _returnvalue 0.0))
  (Audio|Components|Audio|SetVolumeMultiplier _output (Variables|Default|Getmusic%20volume) :!class /Script/Engine.AudioComponent)
  (Variables|Default|SetCurrenMusicRef _output))

(fn ConstructionScript)