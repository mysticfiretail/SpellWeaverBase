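; Deer animal Blueprint that wanders or flees through a simple self-repeating decision loop started on BeginPlay.
; DecideNextAction runs away if ShouldRun is set, otherwise roams when neither hungry nor tired; those flags are only read here.
; Both moves use AIMoveTo to random reachable points, with faster walk speed when fleeing.
; Successful roams repeat after a random delay, flights immediately; failed moves or hungry and tired states end the loop.
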(event Custom|RunAway
  (Variables|/Script/Engine.CharacterMovementComponent|SetMaxWalkSpeed (Variables|Character|GetCharacterMovement) 3e+02)
  (AI|AIMoveTo self (.RandomLocation (AI|Navigation|GetRandomReachablePointinRadius (Transformation|GetActorLocation) (Math|Random|RandomFloatinRange 1e+03 2e+03) 0 0)) 0 5.0 false
    (:OnSuccess
      (CallFunction|DecideNextAction true))))

(event Custom|DecideNextAction
  (params (SkipDelay? :type Boolean))
  (if SkipDelay?
    _
    (else
      (Utilities|FlowControl|Delay (Math|Conversions|ToFloat(Integer) (Math|Random|RandomIntegerinRange 1 3)))))
  (if (Variables|Default|GetShouldRun?)
    (CallFunction|RunAway)
    (elif (not (Variables|Default|GetIsHungry))
      (if (not (Variables|Default|GetIsTired))
        (CallFunction|RandomRoam)))))

(event Custom|RandomRoam
  (Variables|/Script/Engine.CharacterMovementComponent|SetMaxWalkSpeed (Variables|Character|GetCharacterMovement) 1.5e+02)
  (AI|AIMoveTo self (.RandomLocation (AI|Navigation|GetRandomReachablePointinRadius (Transformation|GetActorLocation) 1.5e+03 0 0)) 0 5.0 false
    (:OnSuccess
      (CallFunction|DecideNextAction false))))

(event EventBeginPlay
  (CallFunction|DecideNextAction false))

(event Collision|EventActorBeginOverlap
  (params (OtherActor :type Actor%20Object%20Reference)))

(event EventTick
  (params (DeltaSeconds :type Float%20%28single-precision%29)))

(fn ConstructionScript)